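; Hitbox actor for character combat that displays a strike or hurtbox sphere and applies damage on contact.
; SpawnHitbox colors the sphere by hitbox type, moves it to the set location, reveals it, then runs a one-shot overlap check.
; CheckCollision damages overlapping ProjectB3Characters other than the owner, whatever the hitbox type.
; A positive launch amount knocks targets away, with direction signed by relative Y position.
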(event `SpawnHitbox`
  (switch `EHitboxEnum` (`self.hitboxType`)
    (:`Strike`
      (`PrimitiveComponent.SetMaterial` (`self.Sphere`) 0 "/AnimationSharing/AnimSharingRed.AnimSharingRed"))
    (:`Hurtbox`
      (`PrimitiveComponent.SetMaterial` (`self.Sphere`) 0 "/AnimationSharing/AnimSharingGreen.AnimSharingGreen")))
  (`SceneComponent.K2_SetWorldLocation` (`self.Sphere`) (`self.hitboxLocation`) false false)
  (`SceneComponent.SetVisibility` (`self.Sphere`) true false)
  (`self.CheckCollision`))

(event `CheckCollision`
  (bind (_returnvalue_x _returnvalue_y) (`KismetMathLibrary.BreakVector` (`self.K2_GetActorLocation`)))
  (bind _launchamount (`self.launchAmount`))
  (for _array_element (`self.GetOverlappingActors` "/Script/ProjectB3.ProjectB3Character")
    (if (!= _array_element (`self.GetOwner`))
      (bind _asproject_b3character (cast `ProjectB3Character` _array_element))
      (`ProjectB3Character.TakeDamage` _asproject_b3character (`self.hitboxDamage`))
      (if (> _launchamount 0.0)
        (bind (_returnvalue_x_2 _returnvalue_y_2) (`KismetMathLibrary.BreakVector` (`self.K2_GetActorLocation` _asproject_b3character)))
        (if (<= _returnvalue_y _returnvalue_y_2)
          (`ProjectB3Character.handleLaunch` _asproject_b3character _launchamount)
          (else
            (`ProjectB3Character.handleLaunch` _asproject_b3character (* -1 _launchamount))))))))

(fn `UserConstructionScript`)