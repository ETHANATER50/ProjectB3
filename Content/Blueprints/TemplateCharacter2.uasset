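; Local multiplayer input router that forwards controls for players 2 to 4 to their characters in a platform-fighter-style game.
; SetCharacterReferences sorts the game mode's Players array into four references by PlayerNumber.
; Per-player input bindings call jump, move right and standard attack on valid references, with forward smash split into ForwardAttack on press and ForwardSmash on release.
; Player 1's reference is stored, but no input here drives it.
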(event `self.ReceiveBeginPlay`)

(event `/Game/Blueprints/BaseCharacterInterface.SetCharacterReferences`
  (bind _asproject_b3game_mode (cast `ProjectB3GameMode` (`GameplayStatics.GetGameMode`)))
  (for _array_element (`ProjectB3GameMode.players` _asproject_b3game_mode)
    (switch `int` (`ProjectB3Character.playerNumber` _array_element)
      (:`0`
        (set `self.Player1Reference` _array_element))
      (:`1`
        (set `self.Player2Reference` _array_element))
      (:`2`
        (set `self.Player3Reference` _array_element))
      (:`3`
        (set `self.Player4Reference` _array_element)))))

(event `InputAction|JumpP4`
  (params (Key :type "Key Structure"))
  ;[1 1 1] Player 4 Controls
  (:`Pressed`
    (bind _player4reference (`self.Player4Reference`)
      (:`then`
        (`self.Jump` _player4reference))
      (:`else`)))
  (:`Released`
    (bind _player4reference_2 (`self.Player4Reference`)
      (:`then`
        (`self.StopJumping` _player4reference_2))
      (:`else`))))

(event `InputAction|JumpP3`
  (params (Key :type "Key Structure"))
  ;[1 1 1] Player 3 Controls
  (:`Pressed`
    (bind _player3reference (`self.Player3Reference`)
      (:`then`
        (`self.Jump` _player3reference))
      (:`else`)))
  (:`Released`
    (bind _player3reference_2 (`self.Player3Reference`)
      (:`then`
        (`self.StopJumping` _player3reference_2))
      (:`else`))))

(event `InputAction|JumpP2`
  (params (Key :type "Key Structure"))
  ;[1 1 1] Player 2 Controls
  (:`Pressed`
    (bind _player2reference (`self.Player2Reference`)
      (:`then`
        (`self.Jump` _player2reference))
      (:`else`)))
  (:`Released`
    (bind _player2reference_2 (`self.Player2Reference`)
      (:`then`
        (`self.StopJumping` _player2reference_2))
      (:`else`))))

(event `InputAction|StandardAttackP3`
  (params (Key :type "Key Structure"))
  ;[1 1 1] Player 3 Controls
  (:`Pressed`
    (bind _player3reference (`self.Player3Reference`)
      (:`then`
        (`self.standardAttack` _player3reference))
      (:`else`))))

(event `InputAction|StandardAttackP4`
  (params (Key :type "Key Structure"))
  ;[1 1 1] Player 4 Controls
  (:`Pressed`
    (bind _player4reference (`self.Player4Reference`)
      (:`then`
        (`self.standardAttack` _player4reference))
      (:`else`))))

(event `InputAction|StandardAttackP2`
  (params (Key :type "Key Structure"))
  ;[1 1 1] Player 2 Controls
  (:`Pressed`
    (bind _player2reference (`self.Player2Reference`)
      (:`then`
        (`self.standardAttack` _player2reference))
      (:`else`))))

(event `InputAction|ForwardSmashP2`
  (params (Key :type "Key Structure"))
  ;[1 1 1] Player 2 Controls
  (:`Pressed`
    (bind _player2reference (`self.Player2Reference`)
      (:`then`
        (`self.forwardAttack` _player2reference))
      (:`else`)))
  (:`Released`
    (bind _player2reference_2 (`self.Player2Reference`)
      (:`then`
        (`self.forwardSmash` _player2reference_2))
      (:`else`))))

(event `InputAction|ForwardSmashP3`
  (params (Key :type "Key Structure"))
  ;[1 1 1] Player 3 Controls
  (:`Pressed`
    (bind _player3reference (`self.Player3Reference`)
      (:`then`
        (`self.forwardAttack` _player3reference))
      (:`else`)))
  (:`Released`
    (bind _player3reference_2 (`self.Player3Reference`)
      (:`then`
        (`self.forwardSmash` _player3reference_2))
      (:`else`))))

(event `InputAction|ForwardSmashP4`
  (params (Key :type "Key Structure"))
  ;[1 1 1] Player 4 Controls
  (:`Pressed`
    (bind _player4reference (`self.Player4Reference`)
      (:`then`
        (`self.forwardAttack` _player4reference))
      (:`else`)))
  (:`Released`
    (bind _player4reference_2 (`self.Player4Reference`)
      (:`then`
        (`self.forwardSmash` _player4reference_2))
      (:`else`))))

(event `InputAxis|MoveRightP3`
  (params (AxisValue :type "Float (single-precision)"))
  ;[1 1 1] Player 3 Controls
  (bind _player3reference (`self.Player3Reference`)
    (:`then`
      (`self.MoveRight` _player3reference AxisValue))
    (:`else`)))

(event `InputAxis|MoveRightP2`
  (params (AxisValue :type "Float (single-precision)"))
  ;[1 1 1] Player 2 Controls
  (bind _player2reference (`self.Player2Reference`)
    (:`then`
      (`self.MoveRight` _player2reference AxisValue))
    (:`else`)))

(event `InputAxis|MoveRightP4`
  (params (AxisValue :type "Float (single-precision)"))
  ;[1 1 1] Player 4 Controls
  (bind _player4reference (`self.Player4Reference`)
    (:`then`
      (`self.MoveRight` _player4reference AxisValue))
    (:`else`)))

(fn `UserConstructionScript`)