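; Game mode that spawns and possesses player characters at PlayerStarts when play begins.
; BeginPlay spawns the first player's character, chosen by the game instance's first Classes entry, for controller 0, then calls SpawnPlayer in a NumPlayers-driven loop.
; SpawnPlayer creates a BasePlayerController and character from that same entry at a start not yet tagged "Taken".
; Characters get their Players array index as PlayerNumber, and all receive SetCharacterReferencesMessage after each SpawnPlayer call.
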(event `self.ReceiveBeginPlay`
  (bind _returnvalue (`GameplayStatics.GetPlayerController` 0))
  (bind _returnvalue_2 (`GameplayStatics.GetPlayerController` 0))
  (bind _asbase_game_instance (cast `BaseGameInstance` (`GameplayStatics.GetGameInstance`)))
  (set `self.GameInstanceReference` _asbase_game_instance)
  (bind _outactors (`GameplayStatics.GetAllActorsOfClass` "/Script/Engine.PlayerStart"))
  (bind _output (`|GetArrayItem` _outactors))
  (`/Engine/EditorBlueprintResources/StandardMacros.IsValid` _output
    (:`Is Valid`
      (set `PlayerStart.PlayerStartTag` "Taken" _output)
      (bind _gameinstancereference (`self.GameInstanceReference`)
        (:`then`
          (switch `CharacterClass` (`|GetArrayItem` (`BaseGameInstance.classes` _gameinstancereference))
            (:`VE_Default`
              (bind _returnvalue_3 (`self.GetTransform` _output))
              (bind _returnvalue_4 (`|SpawnActorFromClass` "/Game/Blueprints/TemplateCharacterBP.TemplateCharacterBP_C" _returnvalue_3 "Undefined" "OverrideRootScale" null null))
              (`Controller.UnPossess` _returnvalue)
              (`Controller.Possess` _returnvalue _returnvalue_4)
              (bind _returnvalue_5 (`KismetArrayLibrary.Array_Add` (`self.players`) _returnvalue_4))
              (set `ProjectB3Character.playerNumber` _returnvalue_5 _returnvalue_4))
            (:`VE_Default2`
              (bind _returnvalue_6 (`|SpawnActorFromClass` "/Game/Blueprints/TemplateCharacter2.TemplateCharacter2_C" _returnvalue_3 "Undefined" "OverrideRootScale" null null))
              (`Controller.UnPossess` _returnvalue_2)
              (`Controller.Possess` _returnvalue_2 _returnvalue_6)
              (bind _returnvalue_7 (`KismetArrayLibrary.Array_Add` (`self.players`) _returnvalue_6))
              (set `ProjectB3Character.playerNumber` _returnvalue_7 _returnvalue_6)))
          (for _ (range (`self.numPlayers`))
            (`self.SpawnPlayer`)
            (for _array_element (`self.players`)
              (message `/Game/Blueprints/BaseCharacterInterface.SetCharacterReferences` _array_element))))
        (:`else`)))))

(fn `SpawnPlayer`
  (bind _outactors (`GameplayStatics.GetAllActorsOfClass` "/Script/Engine.PlayerStart"))
  (for _array_element _outactors
    (if (!= (`PlayerStart.PlayerStartTag` _array_element) "Taken")
      (bind _returnvalue (`self.GetTransform` _array_element))
      (bind _returnvalue_2 (`|SpawnActorFromClass` "/Script/ProjectB3.BasePlayerController" _returnvalue "Undefined" "OverrideRootScale" null null))
      (switch `CharacterClass` (`|GetArrayItem` (`BaseGameInstance.classes` (`self.GameInstanceReference`)))
        (:`VE_Default`
          (bind _returnvalue_3 (`|SpawnActorFromClass` "/Game/Blueprints/TemplateCharacterBP.TemplateCharacterBP_C" _returnvalue "Undefined" "OverrideRootScale" null null))
          (`KismetSystemLibrary.PrintString` "Player Spawned!")
          (`Controller.Possess` _returnvalue_2 _returnvalue_3)
          (set `PlayerStart.PlayerStartTag` "Taken" _array_element)
          (bind _returnvalue_4 (`KismetArrayLibrary.Array_Add` (`self.players`) _returnvalue_3))
          (set `ProjectB3Character.playerNumber` _returnvalue_4 _returnvalue_3)
          (break))
        (:`VE_Default2`
          (bind _returnvalue_5 (`|SpawnActorFromClass` "/Game/Blueprints/TemplateCharacter2.TemplateCharacter2_C" _returnvalue "Undefined" "OverrideRootScale" null null))
          (`KismetSystemLibrary.PrintString` "Player Spawned!")
          (`Controller.Possess` _returnvalue_2 _returnvalue_5)
          (set `PlayerStart.PlayerStartTag` "Taken" _array_element)
          (bind _returnvalue_6 (`KismetArrayLibrary.Array_Add` (`self.players`) _returnvalue_5))
          (set `ProjectB3Character.playerNumber` _returnvalue_6 _returnvalue_5)
          (break))))))

(fn `UserConstructionScript`)